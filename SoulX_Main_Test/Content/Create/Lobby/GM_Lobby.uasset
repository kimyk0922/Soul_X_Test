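; GM_Lobby is the lobby Blueprint that shows the WG_Lobby widget and sends the player into a random level on click.
; BeginPlay enables input, adds the widget and resets a DoOnce, which the IA_Cilck action enters.
; The first click removes the widget, prints and opens a random Level array entry, re-rolled per node, so log and destination can differ.
; IA_Cancel is empty, and its right-click logic is disconnected.
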(event Input|EnhancedActionEvents|EnhancedInputActionIA_Cilck
  (params (ActionValue :type Boolean) (ElapsedSeconds :type Float%20%28double-precision%29) (TriggeredSeconds :type Float%20%28double-precision%29) (InputAction :type Input%20Action%20Object%20Reference :default "/Game/Create/Lobby/Input/IA_Cilck.IA_Cilck"))
  (bind _level (Variables|Default|GetLevel))
  (bind (_outitem _outindex) (Utilities|Array|Random _level))
  (Development|PrintString "Left_Click" true true "(R=0.000000,G=0.660000,B=1.000000,A=1.000000)" 5.0)
  (Utilities|FlowControl|DoOnce false
    (:Completed
      (Widget|RemovefromParent (stale EventBeginPlay _returnvalue))
      (Development|PrintString (Utilities|String|Append "Level : " (Utilities|String|ToString(Name) _outitem) "" "Index : " (Utilities|String|ToString(Integer) _outindex)) true true "(R=0.554979,G=0.030354,B=1.000000,A=1.000000)" 5.0)
      (Game|OpenLevel(byName) _outitem))))

(event Input|EnhancedActionEvents|EnhancedInputActionIA_Cancel
  (params (ActionValue :type Boolean) (ElapsedSeconds :type Float%20%28double-precision%29) (TriggeredSeconds :type Float%20%28double-precision%29) (InputAction :type Input%20Action%20Object%20Reference :default "/Game/Create/Lobby/Input/IA_Cancel.IA_Cancel")))

(event EventBeginPlay
  (bind _level (Variables|Default|GetLevel))
  (bind (_outitem _outindex) (Utilities|Array|Random _level))
  (Utilities|FlowControl|Sequence
    (:then_0
      (Input|EnableInput (Game|GetPlayerController 0))
      (bind _returnvalue (UserInterface|CreateWidget "/Game/Create/Lobby/Widget/WG_Lobby.WG_Lobby_C"))
      (UserInterface|Viewport|AddtoViewport _returnvalue 0))
    (:then_1
      (Utilities|FlowControl|DoOnce false) ; enters at Reset
    )))

(fn ConstructionScript)